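; Map is a self-replicating level segment for a platforming course that extends itself as the player advances.
; Its construction script randomizes the sideways (local Y) position of four child actors and a Shrimp component, varying each segment's layout.
; When BP_ThirdPersonCharacter first overlaps the Nexmaca trigger, a DoOnce spawns another Map at the Nexma component's transform, chaining segments endlessly.
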(event OnComponentBeginOverlap(nexmaca)
  (params (OverlappedComponent :type Primitive%20Component%20Object%20Reference) (OtherActor :type Actor%20Object%20Reference) (OtherComp :type Primitive%20Component%20Object%20Reference) (OtherBodyIndex :type Integer) (bFromSweep :type Boolean) (SweepResult :type Hit%20Result%20Structure%20%28by%20ref%29))
  (Utilities|Casting|CastToBP_ThirdPersonCharacter OtherActor)
  (Utilities|FlowControl|DoOnce false
    (:Completed
      (Game|SpawnActorfromClass "Map_C" (Transformation|GetWorldTransform (Variables|Default|Getnexma)) "Undefined" "MultiplyWithRoot" 0 0))))

(event EventBeginPlay)

(event Collision|EventActorBeginOverlap
  (params (OtherActor :type Actor%20Object%20Reference)))

(event EventTick
  (params (DeltaSeconds :type Float%20%28single-precision%29)))

(fn ConstructionScript
  (bind _childactor (Variables|Default|GetChildActor))
  (bind _childactor1 (Variables|Default|GetChildActor1))
  (bind _childactor3 (Variables|Default|GetChildActor3))
  (bind _shrimp (Variables|Default|GetShrimp))
  (bind _childactor2 (Variables|Default|GetChildActor2))
  (bind _relativelocation (Variables|/Script/Engine.SceneComponent|GetRelativeLocation _childactor))
  (bind _relativelocation_2 (Variables|/Script/Engine.SceneComponent|GetRelativeLocation _childactor1))
  (bind _relativelocation_3 (Variables|/Script/Engine.SceneComponent|GetRelativeLocation _childactor3))
  (bind _relativelocation_4 (Variables|/Script/Engine.SceneComponent|GetRelativeLocation _childactor2))
  (bind _relativelocation_5 (Variables|/Script/Engine.SceneComponent|GetRelativeLocation _shrimp))
  (Transformation|SetRelativeLocation _childactor (Math|Vector|MakeVector (.x _relativelocation) (Math|Random|RandomFloatinRange -1e+02 1e+02) (.z _relativelocation)) false false)
  (Transformation|SetRelativeLocation _childactor2 (Math|Vector|MakeVector (.x _relativelocation_4) (Math|Random|RandomFloatinRange -2e+02 2e+02) (.z _relativelocation_4)) false false)
  (Transformation|SetRelativeLocation _childactor1 (Math|Vector|MakeVector (.x _relativelocation_2) (Math|Random|RandomFloatinRange -1e+02 1e+02) (.z _relativelocation_2)) false false)
  (Transformation|SetRelativeLocation _childactor3 (Math|Vector|MakeVector (.x _relativelocation_3) (Math|Random|RandomFloatinRange -2e+02 2e+02) (.z _relativelocation_3)) false false)
  (Transformation|SetRelativeLocation _shrimp (Math|Vector|MakeVector (.x _relativelocation_5) (Math|Random|RandomFloatinRange -1.5e+02 1.5e+02) (.z _relativelocation_5)) false false))