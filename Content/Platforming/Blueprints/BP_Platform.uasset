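; BP_Platform is a moving bounce platform that launches the player character upward.
; The construction script gives InterpToMovement two relative control points, from the origin to MoveToPos.
; When BP_ThirdPersonCharacter begins overlapping the Cube without upward velocity, it is launched with a fixed vertical velocity that overrides only Z.
; Upward-moving characters pass without a launch, and both cases print a debug string.
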(event OnComponentBeginOverlap(Cube)
  (params (OverlappedComponent :type Primitive%20Component%20Object%20Reference) (OtherActor :type Actor%20Object%20Reference) (OtherComp :type Primitive%20Component%20Object%20Reference) (OtherBodyIndex :type Integer) (bFromSweep :type Boolean) (SweepResult :type Hit%20Result%20Structure%20%28by%20ref%29))
  (bind _asbp_third_person_character (Utilities|Casting|CastToBP_ThirdPersonCharacter OtherActor))
  (if (> (.z (Transformation|GetVelocity _asbp_third_person_character)) 0.0)
    (Development|PrintString "jump")
    (else
      (Development|PrintString "fall")
      (Character|LaunchCharacter _asbp_third_person_character "0.000000,0.000000,1400.000000" false true))))

(event EventTick
  (params (DeltaSeconds :type Float%20%28single-precision%29)))

(fn ConstructionScript
  (Class|InterptoMovementComponent|AddControlPointPosition (Variables|Default|GetInterpToMovement) "0, 0, 0" true)
  (Class|InterptoMovementComponent|AddControlPointPosition (Variables|Default|GetInterpToMovement) (Variables|Default|GetMoveToPos) true))