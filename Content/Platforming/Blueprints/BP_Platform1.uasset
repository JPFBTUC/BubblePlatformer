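; BP_Platform1 is a moving platform that also acts as a bounce pad for the third-person character.
; The Movement timeline sets the cube's relative location, and a two-second Delay on its Update pin toggles IsLooped to play or reverse it.
; Overlapping characters that are not moving upward get launched vertically.
; The construction script also gives an InterpToMovement component control points at the origin and MoveToPos.
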(event OnComponentBeginOverlap(Cube)
  (params (OverlappedComponent :type Primitive%20Component%20Object%20Reference) (OtherActor :type Actor%20Object%20Reference) (OtherComp :type Primitive%20Component%20Object%20Reference) (OtherBodyIndex :type Integer) (bFromSweep :type Boolean) (SweepResult :type Hit%20Result%20Structure%20%28by%20ref%29))
  (bind _asbp_third_person_character (Utilities|Casting|CastToBP_ThirdPersonCharacter OtherActor))
  (if (not (> (.z (Transformation|GetVelocity _asbp_third_person_character)) 0.0))
    (Character|LaunchCharacter _asbp_third_person_character "0.000000,0.000000,1450.000000" false true)))

(event EventBeginPlay
  (bind _mov (Timeline|Movement Play)
    (:Update
      (Transformation|SetRelativeLocation (Variables|Default|GetCube) _mov false false)
      (Utilities|FlowControl|Delay 2.0)
      (if (Variables|Default|GetIsLooped)
        (Variables|Default|SetIsLooped false)
        (Timeline|Movement Reverse)
        (else
          (Variables|Default|SetIsLooped true)
          (Timeline|Movement Play))))))

(fn ConstructionScript
  (Class|InterptoMovementComponent|AddControlPointPosition (Variables|Default|GetInterpToMovement) "0, 0, 0" true)
  (Class|InterptoMovementComponent|AddControlPointPosition (Variables|Default|GetInterpToMovement) (Variables|Default|GetMoveToPos) true))